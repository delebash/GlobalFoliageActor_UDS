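; Global foliage control actor that syncs foliage wind, season, health and color variation with Ultra Dynamic Weather.
; RunGlobalFoliageActor runs on construction, BeginPlay and EditorUpdate, writing to the foliage and UDW Material Parameter Collections.
; The icon's yaw sets tree, Project Nature and UDW wind direction.
; UDW weather wind intensity, rescaled and offset per system, overrides tree strength and sets Project Nature strength; AWS values are only computed.
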(event EventTick
  (params (DeltaSeconds :type Float%20%28single-precision%29)))

(event EventEditorUpdate
  ;[1 1 1] Added Weather Effects Interface to Class Settings.  When you change UDW Weather Type rerun GFA
  (GlobalWind|RunGlobalFoliageActor))

(event EventBeginPlay
  (GlobalWind|RunGlobalFoliageActor))

(fn ConstructionScript
  (GlobalWind|RunGlobalFoliageActor))

(fn RunGlobalFoliageActor
  (bind _icon_sock (Variables|Default|GetIcon_Sock))
  (bind _icon_root (Variables|Default|GetIcon_Root))
  (bind _tree___flip_wind_direction (Variables|GlobalWind|GetTree%20-%20Flip%20Wind%20Direction))
  (bind _returnvalue (Transformation|GetWorldRotation _icon_root))
  (bind _yaw (Math|Rotator|BreakRotator _returnvalue))
  ;[1 1 1] Wind
  (Utilities|FlowControl|Sequence
    (:then_0
      (if _tree___flip_wind_direction
        ;[1 1 1] Flipped Icon Function
        (Transformation|SetRelativeRotation _icon_sock "0,180.000000, 0" false false)
        (Transformation|SetRelativeLocation _icon_sock "-220.000000, 0, 0" false false) ; fix location of wind sock center to not intersect with the trees
      )
      (if _tree___flip_wind_direction
        (if (< _yaw 0.0)
          (bind _output_get (Variables|Tree-Wind|SetTree%20-%20Wind%20Direction (+ (* (/ (+ _yaw 3.6e+02) 3.6e+02) -1.0) 1.625)))
          (Rendering|Material|SetScalarParameterValue "/Game/MSPresets/MS_Foliage_Material/MaterialParameterCollection/MPC_GlobalFoliageActor.MPC_GlobalFoliageActor" "Wind Direction" _output_get :!class /Script/Engine.KismetMaterialLibrary)
          (else
            (bind _output_get_2 (Variables|Tree-Wind|SetTree%20-%20Wind%20Direction (+ (* (/ _yaw 3.6e+02) -1.0) 1.625)))
            (Rendering|Material|SetScalarParameterValue "/Game/MSPresets/MS_Foliage_Material/MaterialParameterCollection/MPC_GlobalFoliageActor.MPC_GlobalFoliageActor" "Wind Direction" _output_get_2 :!class /Script/Engine.KismetMaterialLibrary)))
        (elif (< _yaw 0.0)
          (bind _output_get_3 (Variables|Tree-Wind|SetTree%20-%20Wind%20Direction (+ (* (/ (+ _yaw 3.6e+02) 3.6e+02) -1.0) 1.125)))
          (Rendering|Material|SetScalarParameterValue "/Game/MSPresets/MS_Foliage_Material/MaterialParameterCollection/MPC_GlobalFoliageActor.MPC_GlobalFoliageActor" "Wind Direction" _output_get_3 :!class /Script/Engine.KismetMaterialLibrary)
          (else
            (bind _output_get_4 (Variables|Tree-Wind|SetTree%20-%20Wind%20Direction (+ (* (/ _yaw 3.6e+02) -1.0) 1.125)))
            (Rendering|Material|SetScalarParameterValue "/Game/MSPresets/MS_Foliage_Material/MaterialParameterCollection/MPC_GlobalFoliageActor.MPC_GlobalFoliageActor" "Wind Direction" _output_get_4 :!class /Script/Engine.KismetMaterialLibrary))))
      ;[1 1 1] Global Foliage Actor
      (Transformation|SetWorldRotation (Variables|Default|GetIcon_Base) "0, 0, 0" false false)
      (Transformation|SetWorldRotation (Variables|Default|GetIcon_Arrow_Test) (Math|Rotator|MakeRotator 0.0 0.0 (.Yaw (Math|Rotator|BreakRotator (Transformation|GetWorldRotation (Variables|Default|GetIcon_Root))))) false false)
      ;[1 1 1] Wind Parameters
      (Rendering|Material|SetScalarParameterValue "/Game/MSPresets/MS_Foliage_Material/MaterialParameterCollection/MPC_GlobalFoliageActor.MPC_GlobalFoliageActor" "Wind Strength" (Variables|Tree-Wind|GetTree%20-%20Wind%20Strength) :!class /Script/Engine.KismetMaterialLibrary)
      (Rendering|Material|SetScalarParameterValue "/Game/MSPresets/MS_Foliage_Material/MaterialParameterCollection/MPC_GlobalFoliageActor.MPC_GlobalFoliageActor" "Wind Speed" (Variables|Tree-Wind|GetTree%20-%20Wind%20Speed) :!class /Script/Engine.KismetMaterialLibrary)
      (Rendering|Material|SetScalarParameterValue "/Game/MSPresets/MS_Foliage_Material/MaterialParameterCollection/MPC_GlobalFoliageActor.MPC_GlobalFoliageActor" "Wind Tiling" (Variables|Tree-Wind|GetTree%20-%20Wind%20Tiling) :!class /Script/Engine.KismetMaterialLibrary)
      (Rendering|Material|SetScalarParameterValue "/Game/MSPresets/MS_Foliage_Material/MaterialParameterCollection/MPC_GlobalFoliageActor.MPC_GlobalFoliageActor" "Wind Noise" (Variables|Tree-Wind|GetTree%20-%20Wind%20Noise) :!class /Script/Engine.KismetMaterialLibrary)
      ;[1 1 1] Season & Health Parameter
      (Rendering|Material|SetScalarParameterValue "/Game/MSPresets/MS_Foliage_Material/MaterialParameterCollection/MPC_GlobalFoliageActor.MPC_GlobalFoliageActor" "Health" (Variables|Season&Health|GetHealth) :!class /Script/Engine.KismetMaterialLibrary)
      (Rendering|Material|SetScalarParameterValue "/Game/MSPresets/MS_Foliage_Material/MaterialParameterCollection/MPC_GlobalFoliageActor.MPC_GlobalFoliageActor" "Season Strength" (Variables|Season&Health|GetSeason%20Strength) :!class /Script/Engine.KismetMaterialLibrary)
      (Rendering|Material|SetScalarParameterValue "/Game/MSPresets/MS_Foliage_Material/MaterialParameterCollection/MPC_GlobalFoliageActor.MPC_GlobalFoliageActor" "Season Saturation" (Variables|Season&Health|GetSeason%20Saturation) :!class /Script/Engine.KismetMaterialLibrary)
      (Rendering|Material|SetScalarParameterValue "/Game/MSPresets/MS_Foliage_Material/MaterialParameterCollection/MPC_GlobalFoliageActor.MPC_GlobalFoliageActor" "Season Brightness" (Variables|Season&Health|GetSeason%20Brightness) :!class /Script/Engine.KismetMaterialLibrary)
      ;[1 1 1] Color Variation
      (Rendering|Material|SetScalarParameterValue "/Game/MSPresets/MS_Foliage_Material/MaterialParameterCollection/MPC_GlobalFoliageActor.MPC_GlobalFoliageActor" "Variation Tiling" (Variables|ColorVariation|GetVariation%20Tiling) :!class /Script/Engine.KismetMaterialLibrary)
      (Rendering|Material|SetScalarParameterValue "/Game/MSPresets/MS_Foliage_Material/MaterialParameterCollection/MPC_GlobalFoliageActor.MPC_GlobalFoliageActor" "Macro Variation Tiling" (Variables|ColorVariation|GetMacro%20Variation%20Tiling) :!class /Script/Engine.KismetMaterialLibrary)
      (Rendering|Material|SetScalarParameterValue "/Game/MSPresets/MS_Foliage_Material/MaterialParameterCollection/MPC_GlobalFoliageActor.MPC_GlobalFoliageActor" "Random Color Variation" (Variables|ColorVariation|GetRandom%20Color%20Variation%20Amount) :!class /Script/Engine.KismetMaterialLibrary)
      (Rendering|Material|SetScalarParameterValue "/Game/MSPresets/MS_Foliage_Material/MaterialParameterCollection/MPC_GlobalFoliageActor.MPC_GlobalFoliageActor" "Overall Color Variation" (Variables|ColorVariation|GetOverall%20Color%20Variation%20Amount) :!class /Script/Engine.KismetMaterialLibrary))
    (:then_1
      ;[1 1 1] Season & Health For Megascan Foliage
      (Rendering|Material|SetScalarParameterValue "/Game/UltraDynamicSky/Materials/Weather/UltraDynamicWeather_Parameters.UltraDynamicWeather_Parameters" "GFA_Health" (Variables|Season&Health|GetHealth) :!class /Script/Engine.KismetMaterialLibrary)
      (Rendering|Material|SetScalarParameterValue "/Game/UltraDynamicSky/Materials/Weather/UltraDynamicWeather_Parameters.UltraDynamicWeather_Parameters" "GFA_Season_Strength" (Variables|Season&Health|GetSeason%20Strength) :!class /Script/Engine.KismetMaterialLibrary)
      (Rendering|Material|SetScalarParameterValue "/Game/UltraDynamicSky/Materials/Weather/UltraDynamicWeather_Parameters.UltraDynamicWeather_Parameters" "GFA_Season_Saturation" (Variables|Season&Health|GetSeason%20Saturation) :!class /Script/Engine.KismetMaterialLibrary)
      (Rendering|Material|SetScalarParameterValue "/Game/UltraDynamicSky/Materials/Weather/UltraDynamicWeather_Parameters.UltraDynamicWeather_Parameters" "GFA_Season_Brightness" (Variables|Season&Health|GetSeason%20Brightness) :!class /Script/Engine.KismetMaterialLibrary))
    (:then_2
      ;[1 1 1] Get UDS Weather Type
      (bind _returnvalue_2 (Actor|GetActorOfClass "/Game/UltraDynamicSky/Blueprints/Ultra_Dynamic_Weather.Ultra_Dynamic_Weather_C"))
      (Variables|UDS-WindWeather|SetUDW _returnvalue_2)
      (Variables|UDS-WindWeather|SetCurrent%20Weather (Variables|/Game/UltraDynamicSky/Blueprints/Ultra_Dynamic_Weather.Ultra_Dynamic_Weather_C|GetWeather (Variables|UDS-WindWeather|GetUDW))))
    (:then_3
      ;[1 1 1] Set local variabels to parameter collection values
      (Variables|UDS-WindWeather|SetUDS%20-Wind%20Intensity (Variables|/Game/UltraDynamicSky/Blueprints/Weather_Effects/System/UDS_Weather_Settings.UDS_Weather_Settings_C|GetWind%20Intensity (Variables|UDS-WindWeather|GetCurrent%20Weather)))
      (bind _returnvalue_3 (Rendering|Material|GetScalarParameterValue "/Game/UltraDynamicSky/Materials/Weather/UltraDynamicWeather_Parameters.UltraDynamicWeather_Parameters" "Wind Angle" :!class /Script/Engine.KismetMaterialLibrary))
      (Variables|UDS-WindWeather|SetUDS%20-%20Wind%20Direction _returnvalue_3)
      (bind _returnvalue_4 (Rendering|Material|GetScalarParameterValue "/Game/MSPresets/MS_Foliage_Material/MaterialParameterCollection/MPC_GlobalFoliageActor.MPC_GlobalFoliageActor" "Wind Direction" :!class /Script/Engine.KismetMaterialLibrary))
      (Variables|Tree-Wind|SetTree%20-%20Wind%20Direction _returnvalue_4)
      (bind _output_get_5 (Variables|GlobalWind|SetWind%20Direction%20%20Icon%20Rotation (.Yaw (Math|Rotator|BreakRotator (Transformation|GetWorldRotation (Variables|Default|GetIcon_Root))))))
      (Variables|UDS-WindWeather|SetUDS%20-%20Wind%20Direction _output_get_5))
    (:then_4
      ;[1 1 1] Adjust Wind Speeds for difference in UDS, PN Foliage,Trees, and ABS  Wind shaders
      (Variables|PN-Wind|SetPN%20-%20Wind%20Intensity%20Adjusted (+ (Variables|UDS-WindWeather|GetUDS%20-Wind%20Intensity) (Variables|GlobalWind|GetFoliage%20-%20Wind%20Intensity%20Offset)))
      (Variables|Tree-Wind|SetTree%20-%20Wind%20Strength%20Adjusted (+ (* (Variables|UDS-WindWeather|GetUDS%20-Wind%20Intensity) 2.0) (Variables|GlobalWind|GetTrees%20-%20Wind%20Intensity%20Offset)))
      (Variables|AWS-Wind|SetAWS%20-%20Physical%20Wind%20Adjusted (+ (/ (Variables|UDS-WindWeather|GetUDS%20-Wind%20Intensity) 1e+01) (Variables|AWS-Wind|GetAWS%20-%20Physical%20Wind%20Offset)))
      (Variables|AWS-Wind|SetAWS%20-%20Cloth%20Speedtree%20Wind%20Adjusted (+ (/ (Variables|UDS-WindWeather|GetUDS%20-Wind%20Intensity) 1e+01) (Variables|AWS-Wind|GetAWS%20-%20Cloth%20Speedtree%20Wind%20Offset)))
      (Variables|AWS-Wind|SetAWS%20-%20Particle%20Wind%20Adjusted (+ (/ (Variables|UDS-WindWeather|GetUDS%20-Wind%20Intensity) 1e+01) (Variables|AWS-Wind|GetAWS%20-%20Particle%20Wind%20Offset))))
    (:then_5
      ;[1 1 1] Update Parameter Collections
      ;;[0.1995 0.2653 1] PN - Project Nature
      (Rendering|Material|SetScalarParameterValue "/Game/UltraDynamicSky/Materials/Weather/UltraDynamicWeather_Parameters.UltraDynamicWeather_Parameters" "PN Wind Strength" (Variables|PN-Wind|GetPN%20-%20Wind%20Intensity%20Adjusted) :!class /Script/Engine.KismetMaterialLibrary)
      (Rendering|Material|SetScalarParameterValue "/Game/UltraDynamicSky/Materials/Weather/UltraDynamicWeather_Parameters.UltraDynamicWeather_Parameters" "PN Wind Direction" (Variables|GlobalWind|GetWind%20Direction%20%20Icon%20Rotation) :!class /Script/Engine.KismetMaterialLibrary)
      ;;[0.3543 1 0.8079] UDS - UDW
      (Variables|/Game/UltraDynamicSky/Blueprints/Ultra_Dynamic_Weather.Ultra_Dynamic_Weather_C|SetWind%20Direction (Variables|UDS-WindWeather|GetUDW) (Variables|UDS-WindWeather|GetUDS%20-%20Wind%20Direction))
      (Rendering|Material|SetScalarParameterValue "/Game/UltraDynamicSky/Materials/Weather/UltraDynamicWeather_Parameters.UltraDynamicWeather_Parameters" "Wind Intensity" (Variables|UDS-WindWeather|GetUDS%20-Wind%20Intensity) :!class /Script/Engine.KismetMaterialLibrary)
      ;;[0.2528 1 0.1602] Trees
      (Rendering|Material|SetScalarParameterValue "/Game/MSPresets/MS_Foliage_Material/MaterialParameterCollection/MPC_GlobalFoliageActor.MPC_GlobalFoliageActor" "Wind Strength" (Variables|Tree-Wind|GetTree%20-%20Wind%20Strength%20Adjusted) :!class /Script/Engine.KismetMaterialLibrary))
    (:then_6)
    (:then_7)))

(fn CheckWaveAssetExists
  (params (AssetName :type String) (AssetFolder :type String))
  ;[1 1 1] Check if Wave Asset Exists
  (Variables|Default|SetAsset%20Folder AssetFolder)
  (Variables|Default|SetAsset%20Name AssetName)
  (bind _returnvalue (Class|AssetRegistry|GetAssetbyObjectPath (Class|AssetRegistryHelpers|GetAssetRegistry) (Utilities|String|StringToName (Utilities|String|Append (Utilities|String|Append (Utilities|String|Append (Utilities|String|Append (Variables|Default|GetAsset%20Folder) "/") (Variables|Default|GetAsset%20Name)) ".") (Variables|Default|GetAsset%20Name))) false))
  (if (Class|AssetRegistryHelpers|IsUAsset _returnvalue)
    (return true)
    (else
      (Development|PrintString (Utilities|String|ToString(Name) (Utilities|String|StringToName (Utilities|String|Append (Utilities|String|Append (Utilities|String|Append (Utilities|String|Append (Variables|Default|GetAsset%20Folder) "/") (Variables|Default|GetAsset%20Name)) ".") (Variables|Default|GetAsset%20Name)))))
      (Development|PrintString "   Asset Not Found"))))