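; Holding Blueprint of unexecuted node graphs that, per its name, are copied to enable UE Water integration, alongside Ambient Wind System wiring.
; Lake and ocean bodies get Gerstner wave assets, optionally named by UDS weather with default fallbacks, though the ocean load uses the lake asset name.
; Wind direction updates the last-processed body's wave generator before recalculation.
; Separate snippets push wind settings to AWS and flowmap speed to river materials.
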(fn CopyInfo)